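; Game mode for a runner game that builds the floor track from tile actors, laying starting tiles and then random tiles at BeginPlay.
; Each spawned tile's SpawnPoint component sets the location of the next, always with zero rotation and unit scale.
; SpawnTile picks randomly from FloorTiles and counts straights; once the count exceeds seven, it spawns a random FloorCorners piece instead, resetting the count.
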(event EventBeginPlay
  (for _index (range 0 4)
    (CallFunction|SpawnFirstTile))
  (for _index_2 (range 0 9)
    (CallFunction|SpawnTile)))

(event EventTick
  (params (DeltaSeconds :type Float%20%28single-precision%29)))

(fn ConstructionScript)

(fn SpawnTile
  (bind _floortiles (Variables|Default|GetFloorTiles))
  (if (> (Variables|Default|GetCurrentStraights) 7)
    (CallFunction|SpawnCorners)
    (else
      (bind _returnvalue (Game|SpawnActorfromClass (Utilities|Array|Get(acopy) _floortiles (Math|Random|RandomIntegerinRange 0 (Utilities|Array|LastIndex _floortiles))) (Variables|Default|GetNextSpawnPoint) "Undefined" 0 0))
      (bind _asmaster_tile (Utilities|Casting|CastToMasterTile _returnvalue))
      (Variables|Default|SetNextSpawnPoint (Math|Transform|MakeTransform (Transformation|GetWorldLocation (Variables|/Script/SkyRunner.MasterTile|GetSpawnPoint _asmaster_tile)) "0, 0, 0" "1,1,1"))
      (Variables|Default|SetCurrentStraights (+ (Variables|Default|GetCurrentStraights) 1)))))

(fn SpawnFirstTile
  (bind _returnvalue (Game|SpawnActorfromClass "/Game/RunnerFiles/BluePrints/BP_FirstTile.BP_FirstTile_C" (Variables|Default|GetNextSpawnPoint) "Undefined" 0 0))
  (Variables|Default|SetNextSpawnPoint (Math|Transform|MakeTransform (Transformation|GetWorldLocation (Variables|/Script/SkyRunner.MasterTile|GetSpawnPoint _returnvalue)) "0, 0, 0" "1,1,1")))

(fn SpawnCorners
  (bind _floorcorners (Variables|Default|GetFloorCorners))
  (bind _returnvalue (Game|SpawnActorfromClass (Utilities|Array|Get(acopy) _floorcorners (Math|Random|RandomIntegerinRange 0 (Utilities|Array|LastIndex _floorcorners))) (Variables|Default|GetNextSpawnPoint) "Undefined" 0 0))
  (bind _asmaster_tile (Utilities|Casting|CastToMasterTile _returnvalue))
  (Variables|Default|SetNextSpawnPoint (Math|Transform|MakeTransform (Transformation|GetWorldLocation (Variables|/Script/SkyRunner.MasterTile|GetSpawnPoint _asmaster_tile)) "0, 0, 0" "1,1,1"))
  (Variables|Default|SetCurrentStraights 0))