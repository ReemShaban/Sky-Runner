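; BP_Boot is a jump-boost pickup for the runner game.
; When a Runner overlaps it, it raises the character's JumpZVelocity and hides its mesh.
; After a ten-second delay it restores a lower jump velocity on player character 0, rather than on the overlapping actor, then destroys itself.
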(event EventBeginPlay)

(event Collision|EventActorBeginOverlap
  (params (OtherActor :type Actor%20Object%20Reference))
  (bind _asrunner (Utilities|Casting|CastToRunner OtherActor))
  (Variables|/Script/Engine.CharacterMovementComponent|SetJumpZVelocity (Variables|/Script/Engine.Character|GetCharacterMovement _asrunner) 9e+02)
  (Rendering|SetVisibility (Variables|Default|GetStaticMesh) false false)
  (Utilities|FlowControl|Delay 1e+01)
  (bind _asrunner_2 (Utilities|Casting|CastToRunner (Game|GetPlayerCharacter 0)))
  (Variables|/Script/Engine.CharacterMovementComponent|SetJumpZVelocity (Variables|/Script/Engine.Character|GetCharacterMovement _asrunner_2) 4.5e+02)
  (Actor|DestroyActor))

(event EventTick
  (params (DeltaSeconds :type Float%20%28single-precision%29)))

(fn ConstructionScript)