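; Base track tile for an endless runner, which calls SpawnObstacles when play begins.
; When the Runner overlaps its Box trigger, it asks BP_RunnerGameMode to spawn another tile and adds multiplier-scaled points.
; The same overlap compounds the player's max walk speed slightly within a clamped range, then the tile destroys itself after a short delay.
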(event OnComponentBeginOverlap(Box)
  (params (OverlappedComponent :type Primitive%20Component%20Object%20Reference) (OtherActor :type Actor%20Object%20Reference) (OtherComp :type Primitive%20Component%20Object%20Reference) (OtherBodyIndex :type Integer) (bFromSweep :type Boolean) (SweepResult :type Hit%20Result%20Structure%20%28by%20ref%29))
  (Utilities|Casting|CastToRunner OtherActor)
  (bind _asbp_runner_game_mode (Utilities|Casting|CastToBP_RunnerGameMode (Game|GetGameMode)))
  (Default|SpawnTile _asbp_runner_game_mode)
  (bind _asbp_runner_game_mode_2 (Utilities|Casting|CastToBP_RunnerGameMode (Game|GetGameMode)))
  (Variables|/Script/SkyRunner.Runner_GameMode|SetCurrentPoints _asbp_runner_game_mode_2 (+ (* 1 (Variables|/Script/SkyRunner.Runner_GameMode|GetPointsMultiplier _asbp_runner_game_mode_2)) (Variables|/Script/SkyRunner.Runner_GameMode|GetCurrentPoints _asbp_runner_game_mode_2)))
  (bind _asrunner (Utilities|Casting|CastToRunner (Game|GetPlayerCharacter 0)))
  (Variables|/Script/Engine.CharacterMovementComponent|SetMaxWalkSpeed (Variables|/Script/Engine.Character|GetCharacterMovement _asrunner) (Math|Float|Clamp(Float) (* (Variables|/Script/Engine.CharacterMovementComponent|GetMaxWalkSpeed (Variables|/Script/Engine.Character|GetCharacterMovement _asrunner)) 1.01) 6e+02 1.2e+03))
  (Utilities|FlowControl|Delay 0.5)
  (Actor|DestroyActor))

(event EventBeginPlay
  (Class|MasterTile|SpawnObstacles))

(event Collision|EventActorBeginOverlap
  (params (OtherActor :type Actor%20Object%20Reference)))

(event EventTick
  (params (DeltaSeconds :type Float%20%28single-precision%29)))

(fn ConstructionScript)